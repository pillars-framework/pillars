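; HogWarp weather Blueprint that applies given weather, time of day and season to the game world and reports current weather.
; UpdateWeather sets default and instant override weather, UpdateTime pins the simulation time factor and keeps the date, and UpdateSeason forces a season refresh.
; RequestWeather passes the current weather to SendWeather, which, like SendTime and SendSeason, is an empty stub here.
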(event EventBeginPlay)

(fn ConstructionScript)

(fn UpdateWeather
  (params (Weather :type String))
  (bind _weathermaster (Class|WeatherMasterComponent|GetWeatherMaster))
  (bind _returnvalue (Utilities|String|StringToName Weather))
  (Class|WeatherMasterComponent|SetDefaultWeather _weathermaster _returnvalue)
  (Class|WeatherMasterComponent|SetOverrideWeather _weathermaster _returnvalue true)
  (Class|WeatherMasterComponent|PopWeatherOverride (Class|PhoenixGameInstance|GetPhoenixGameInstancePure)))

(fn UpdateTime
  (params (Hours :type Integer) (Minutes :type Integer) (Seconds :type Integer))
  (bind _returnvalue (Class|Scheduler|Get))
  (Class|Scheduler|SetSimulationTimeFactorOverride _returnvalue 1.0)
  (Class|Scheduler|SetCurrentTime _returnvalue Hours Minutes Seconds (.month (Class|Scheduler|GetSimulatedTime _returnvalue)) (.day (Class|Scheduler|GetSimulatedTime _returnvalue)) (.year (Class|Scheduler|GetSimulatedTime _returnvalue))))

(fn UpdateSeason
  (params (NewSeason :type Integer))
  (Class|SeasonChanger|SetCurrentSeason (Utilities|Enum|ByteToEnumESeasonEnum (Math|Conversions|ToByte(Integer) NewSeason)))
  (Class|PhoenixGameInstance|ForceSeasonUpdate (Class|PhoenixGameInstance|GetPhoenixGameInstancePure) "Season_Invalid"))

(fn SendTime
  (params (Hour :type Integer) (Minute :type Integer) (Second :type Integer)))

(fn SendSeason
  (params (Season :type Integer)))

(fn SendWeather
  (params (Weather :type String)))

(fn RequestWeather
  (bind _thecurrentweather (Class|WeatherMasterComponent|GetCurrentWeather))
  (Server|SendWeather (Utilities|String|ToString(Name) _thecurrentweather)))