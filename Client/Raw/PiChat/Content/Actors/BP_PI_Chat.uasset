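; Chat actor that creates the W_PI_ChatPanel widget, focuses its input on Enter and auto-scrolls new messages after a short delay.
; FromServer feeds messages into the panel via a dispatcher; commits and settings changes go to FromClient and SaveSettings, both empty stubs here.
; An unfocused panel fades out through a timer and opacity timeline.
; Initialize sets size and text scale, and runs automatically when running with the editor.
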(event Custom|TriggerFadeOut
  ;[1 1 1] Fade Out
  (Utilities|Time|ClearandInvalidateTimerbyHandle (Variables|Default|GetFadeDelayTimerHandle))
  (if (not (Variables|/PiChat/Widgets/W_PI_ChatPanel.W_PI_ChatPanel_C|GetInFocus (Variables|Default|GetUI%20Chat)))
    (bind _returnvalue (Utilities|Time|SetTimerbyEvent (delegate Custom|FadeDelayElapsed) 1e+01))
    (Variables|Default|SetFadeDelayTimerHandle _returnvalue)
    (Default|Show (Variables|Default|GetUI%20Chat))))

(event Custom|OnMessageCommit
  (params (Message :type String))
  ;[1 1 1] Chat Panel
  (Server|FromClient Message))

(event Custom|OnSettingsClosed
  (bind _ui_chat (Variables|Default|GetUI%20Chat))
  ;[1 1 1] Settings
  (Default|HideInput _ui_chat)
  (Server|SaveSettings (Variables|/PiChat/Widgets/W_PI_ChatPanel.W_PI_ChatPanel_C|GetHeight _ui_chat) (Variables|/PiChat/Widgets/W_PI_ChatPanel.W_PI_ChatPanel_C|GetWidth _ui_chat) (Variables|/PiChat/Widgets/W_PI_ChatPanel.W_PI_ChatPanel_C|GetText%20Scale _ui_chat)))

(event Custom|OnMessageAdded
  ;[1 1 1] Message Added
  (CallFunction|TriggerFadeOut)
  (CallFunction|TriggerScroll false))

(event Custom|OnMessageReceived
  (params (Message :type String))
  (Default|AddMessage (Variables|Default|GetUI%20Chat) Message))

(event Custom|FadeDelayElapsed
  ;[1 1 1] Fade Out
  (ChatPanel|FadeOutChat true))

(event Custom|TriggerScroll
  (params (Force :type Boolean))
  ;[1 1 1] Delayed Scroll UI Fix
  (if (or Force (Variables|/PiChat/Widgets/W_PI_ChatPanel.W_PI_ChatPanel_C|GetAutoScrollActive (Variables|Default|GetUI%20Chat)))
    (Utilities|FlowControl|Delay 0.1)
    (Default|ScrolltoBottom (Variables|Default|GetUI%20Chat))))

(event Custom|OnInputHidden
  ;[1 1 1] Input Hidden
  (CallFunction|TriggerFadeOut)
  (CallFunction|TriggerScroll false))

(event EventBeginPlay
  (bind _returnvalue (Game|GetPlayerController 0))
  (EventDispatchers|BindEventtoMessageReceived (delegate Custom|OnMessageReceived))
  ;[1 1 1] Chat Panel
  (Input|EnableInput _returnvalue)
  (bind _returnvalue_2 (UserInterface|CreateWidget "/PiChat/Widgets/W_PI_ChatPanel.W_PI_ChatPanel_C" _returnvalue))
  (bind _output_get (Variables|Default|SetUI%20Chat _returnvalue_2))
  (UserInterface|Viewport|AddtoViewport _output_get 1000)
  (Widget|SetVisibility _output_get "Collapsed")
  (EventDispatchers|BindEventtoMessageCommit _output_get (delegate Custom|OnMessageCommit))
  ;[1 1 1] Settings
  (EventDispatchers|BindEventtoSettingsClosed (Variables|Default|GetUI%20Chat) (delegate Custom|OnSettingsClosed))
  ;[1 1 1] Message Added
  (EventDispatchers|BindEventtoMessageAdded (Variables|Default|GetUI%20Chat) (delegate Custom|OnMessageAdded))
  ;[1 1 1] Input Hidden
  (EventDispatchers|BindEventtoInputHidden (Variables|Default|GetUI%20Chat) (delegate Custom|OnInputHidden))
  ;[1 1 1] Editor
  (bind _returnvalue_3 (Class|PhoenixBPLibrary|AvaIsRunningwithEditor))
  (if _returnvalue_3
    (Client|Initialize 4.5e+02 4e+02 2.0)))

(event EventDestroyed
  (bind _ui_chat (Variables|Default|GetUI%20Chat))
  ;[1 1 1] Cleanup
  (Utilities|IsValid _ui_chat
    (:Is%20Valid
      (Widget|RemovefromParent _ui_chat))))

(event Input|KeyboardEvents|Enter
  (params (Key :type Key%20Structure :default "None"))
  ;[1 1 1] On Enter
  (:Pressed
    (if (Variables|/PiChat/Widgets/W_PI_ChatPanel.W_PI_ChatPanel_C|GetIsInitialized (Variables|Default|GetUI%20Chat))
      (ChatPanel|FadeOutChat false)
      (Default|FocusInput (Variables|Default|GetUI%20Chat))
      (CallFunction|TriggerScroll false))))

(fn ConstructionScript)

(fn FromClient
  (params (message :type String)))

(fn FromServer
  (params (message :type String))
  (Default|CallMessageReceived message))

(fn SaveSettings
  (params (height :type Float%20%28single-precision%29) (width :type Float%20%28single-precision%29) (textScale :type Float%20%28single-precision%29)))

(fn Initialize
  (params (height :type Float%20%28single-precision%29) (width :type Float%20%28single-precision%29) (textScale :type Float%20%28single-precision%29))
  (Default|Initialize (Variables|Default|GetUI%20Chat) height width textScale)
  (Default|CallMessageReceived "--- Chat Initialized ---"))

(fn AddMessage
  (params (Message :type String))
  (bind _ui_chat (Variables|Default|GetUI%20Chat))
  (Default|AddMessage _ui_chat Message)
  (if (Variables|/PiChat/Widgets/W_PI_ChatPanel.W_PI_ChatPanel_C|GetIsInitialized _ui_chat)
    (Default|Show (Variables|Default|GetUI%20Chat))
    (return)))

(fn FadeOutChat
  (params (Toggle :type Boolean))
  (bind _fadeoutchattimeline (Variables|Default|GetFadeOutChatTimeLine))
  (if Toggle
    (Components|Timeline|PlayfromStart _fadeoutchattimeline)
    (else
      (Utilities|Time|ClearandInvalidateTimerbyHandle (Variables|Default|GetFadeDelayTimerHandle))
      (Audio|Components|Audio|Stop _fadeoutchattimeline))))