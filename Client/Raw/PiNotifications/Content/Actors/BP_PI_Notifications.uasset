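; BP_PI_Notifications is an actor that shows on-screen notifications through a W_PI_NotificationPanel widget.
; It adds the panel to the viewport on BeginPlay and removes it when destroyed.
; TriggerNotification passes icon, title, message and duration to the panel and posts a Wwise popup sound at the world origin.
; An Enter key handler fires a random test notification when running with the editor.
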(event EventBeginPlay
  (bind _returnvalue (UserInterface|CreateWidget "/PiNotifications/Widgets/W_PI_NotificationPanel.W_PI_NotificationPanel_C" (Game|GetPlayerController 0)))
  (bind _output_get (Variables|Default|SetNotification%20Panel _returnvalue))
  (UserInterface|Viewport|AddtoViewport _output_get 0)
  (Widget|SetVisibility _output_get "Visible"))

(event EventDestroyed
  (bind _notification_panel (Variables|Default|GetNotification%20Panel))
  (Utilities|IsValid _notification_panel
    (:Is%20Valid
      (Widget|RemovefromParent _notification_panel))))

(event Input|KeyboardEvents|Enter
  (params (Key :type Key%20Structure :default "None"))
  (bind _returnvalue (Math|Random|RandomInteger 22))
  (:Pressed
    (bind _returnvalue_2 (Class|PhoenixBPLibrary|AvaIsRunningwithEditor))
    (if _returnvalue_2
      (Client|TriggerNotification _returnvalue (Utilities|String|ToString(Integer) _returnvalue) "Short text" 5.0))))

(fn ConstructionScript)

(fn TriggerNotification
  (params (iconIdx :type Integer) (title :type String) (message :type String) (duration :type Float%20%28single-precision%29))
  (Default|AddNotification (Variables|Default|GetNotification%20Panel) title message duration iconIdx)
  (Class|AkGameplayStatics|PostEventatLocation "/Game/WWise/Events/ui/Inventory/UI_Notification_Item_Popup.UI_Notification_Item_Popup" "0, 0, 0" "0, 0, 0"))